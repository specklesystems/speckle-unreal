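; Speckle converter Blueprint that turns View3D objects into camera actors spawned in the Unreal world.
; CanConvertToNative checks the supported type list, and ConvertToNative casts to View3D and passes it to ViewToNative.
; ViewToNative negates Y on origin, forward and up vectors to convert right-handed to left-handed coordinates, then sets orthographic or perspective projection.
; ConvertToSpeckle is an empty stub, so conversion is one-way.
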(fn `CanConvertToNative`
  (params (BaseType :type "Base Class Reference"))
  (returns (ReturnValue :type Boolean))
  (return (`BlueprintSetLibrary.Set_Contains` (`self.SpeckleTypes`) BaseType)))

(fn `ConvertToNative`
  (params (SpeckleBase :type "Base Object Reference") (World :type "World Object Reference") (AvailableConverters :type "SpeckleConverter Interface (by ref)"))
  (returns (ReturnValue :type "Object Object Reference"))
  (bind _asview_3d (cast `View3D` SpeckleBase)
    (:`then`
      (bind _actor (`self.ViewToNative` _asview_3d World))
      (return _actor))
    (:`CastFailed`
      (return null))))

(fn `ConvertToSpeckle`
  (params (Object :type "Object Object Reference"))
  (returns (ReturnValue :type "Base Object Reference"))
  (return null))

(fn `ViewToNative`
  (params (View :type "View3D Object Reference") (World :type "World Object Reference"))
  (returns (Actor :type "CameraActor Object Reference"))
  (bind _returnvalue (`KismetMathLibrary.MakeVector` 1.0 -1.0 1.0))
  ;[1 0.7557 0.651] Create Actor
  (bind _returnvalue_2 (`SpeckleObjectUtils.SpawnActorInWorld` World (`self.ActorType`) (`KismetMathLibrary.MakeTransform` (* (`View3D.Origin` View) _returnvalue) (`KismetMathLibrary.MakeRotFromXZ` (* (`View3D.ForwardDirection` View) _returnvalue) (* (`View3D.UpDirection` View) _returnvalue)))))
  ;[0.598 0.7655 1] Set Projection Mode
  (if (`View3D.IsOrthogonal` View)
    (bind _cameracomponent (`CameraActor.CameraComponent` _returnvalue_2))
    (`CameraComponent.SetProjectionMode` _cameracomponent "Orthographic")
    (else
      (`CameraComponent.SetProjectionMode` _cameracomponent "Perspective")))
  (return _returnvalue_2))