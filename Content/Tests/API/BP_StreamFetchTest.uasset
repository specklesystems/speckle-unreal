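; BP_StreamFetchTest is an API functional test that checks fetching streams from a server using a URL and auth token.
; On start, it runs an async ReceiveStreamsOperation with a limit, then searches the returned streams for the expected test stream ID.
; It succeeds only if that stream is present and the count stays within the limit, otherwise reporting a failure or the operation's error message.
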(event `self.ReceiveStartTest`
  (set `self.StreamFound` false)
  (bind (_streams _errormessage) (`ReceiveStreamsOperation.ReceiveStreamsOperation` (`self.ServerUrl`) (`self.AuthToken`) (`self.Limit`))
    (:`OnReceiveSuccessfully`
      ;[1 1 1] Check streams contains our specified stream
      (for _array_element _streams
        (if (`KismetStringLibrary.EqualEqual_StrStr` (`.ID` (break `SpeckleStream` _array_element)) (`self.TestStreamId`))
          (set `self.StreamFound` true)
          (break)))
      (if (`self.StreamFound`)
        (set `self.StreamFound` false)
        (bind _returnvalue (`KismetArrayLibrary.Array_Length` _streams))
        ;[1 1 1] Test we did not exceed limit
        (if (>= (`self.Limit`) _returnvalue)
          ;[0.2344 1 0.3365] PASSED
          (`self.FinishTest` "Succeeded" "Successfully recieved stream")
          (else
            ;[1 0.2344 0.2344] FAILED - Recieved more than limit
            (`self.FinishTest` "Failed" (`KismetTextLibrary.Conv_TextToString` (`|FormatText` "Request was sent with a limit of {limit} items, but we recieved more {count}" (`self.Limit`) _returnvalue)))))
        (else
          ;[1 0.2344 0.2344] FAILED Stream not found
          (`self.FinishTest` "Failed" (`KismetTextLibrary.Conv_TextToString` (`|FormatText` "{Count} streams recieved, none with expected id {id}" _returnvalue (`self.TestStreamId`)))))))
    (:`OnError`
      ;[1 0.2344 0.2344] FAILED operation error
      (`self.FinishTest` "Error" _errormessage))))

(fn `UserConstructionScript`)