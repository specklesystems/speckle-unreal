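; BP_UserFetch is a functional test for the API that fetches the current user's data from a server.
; On StartTest it runs an async ReceiveMyUserDataOperation with a server URL and auth token, then prints the returned profile fields.
; It passes when the returned Bio equals TestBio, although the failure message and comments refer to email.
; An operation error finishes the test with an Error result and the operation's message.
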(event `self.ReceiveStartTest`
  (bind (_myuserdata _errormessage) (`ReceiveMyUserDataOperation.ReceiveMyUserDataOperation` (`self.ServerUrl`) (`self.AuthToken`))
    (:`OnReceiveSuccessfully`
      (bind (_id _email _name _bio _company _avatar _role) (break `SpeckleUser` _myuserdata))
      (`KismetSystemLibrary.PrintString` (`KismetTextLibrary.Conv_TextToString` (`|FormatText` "id: {id}, Email: {email}, Name {name}, Bio {Bio}, Company {comapny}, Role {role}" _id _email _name _bio _company _role)))
      ;[1 1 1] Test email matches expected
      (if (`KismetStringLibrary.EqualEqual_StrStr` (`self.TestBio`) _bio)
        ;[0.2344 1 0.3365] PASSED
        (`self.FinishTest` "Succeeded" "Successfully received user info")
        (else
          ;[1 0.2344 0.2344] FAILED - Email does not match
          (`self.FinishTest` "Failed" (`KismetTextLibrary.Conv_TextToString` (`|FormatText` "Fetched user email doesn't match. Expected \"{expected}\", got \"{actual}\"" (`self.TestBio`) _bio))))))
    (:`OnError`
      ;[1 0.2344 0.2344] FAILED operation error
      (`self.FinishTest` "Error" _errormessage))))

(fn `UserConstructionScript`)