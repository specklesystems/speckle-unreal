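; BP_CommitFetchTest is a functional test for fetching commits from a server stream branch through the API.
; On start it runs the async ReceiveCommitsOperation with the configured server, auth token, stream, branch and limit.
; It passes if the returned commits include the expected test commit ID and their count stays within the limit.
; A missing commit or exceeded limit fails the test, while an operation error finishes it with an Error result.
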(event `self.ReceiveStartTest`
  (set `self.CommitFound` false)
  (bind (_commits _errormessage) (`ReceiveCommitsOperation.ReceiveCommitsOperation` (`self.ServerUrl`) (`self.AuthToken`) (`self.StreamId`) (`self.BranchName`) (`self.Limit`))
    (:`OnReceiveSuccessfully`
      ;[1 1 1] Check streams contains our specified stream
      (for _array_element _commits
        (if (`KismetStringLibrary.EqualEqual_StrStr` (`.ID` (break `SpeckleCommit` _array_element)) (`self.TestCommitId`))
          (set `self.CommitFound` true)
          (break)))
      (if (`self.CommitFound`)
        (set `self.CommitFound` false)
        (bind _returnvalue (`KismetArrayLibrary.Array_Length` _commits))
        ;[1 1 1] Test we did not exceed limit
        (if (>= (`self.Limit`) _returnvalue)
          ;[0.2344 1 0.3365] PASSED
          (`self.FinishTest` "Succeeded" "Successfully recieved Commit")
          (else
            ;[1 0.2344 0.2344] FAILED - Recieved more than limit
            (`self.FinishTest` "Failed" (`KismetTextLibrary.Conv_TextToString` (`|FormatText` "Request was sent with a limit of {limit} items, but we recieved more {count}" (`self.Limit`) _returnvalue)))))
        (else
          ;[1 0.2344 0.2344] FAILED Branch not found
          (`self.FinishTest` "Failed" (`KismetTextLibrary.Conv_TextToString` (`|FormatText` "{Count} commits recieved, none with expected id {id}" _returnvalue (`self.TestCommitId`)))))))
    (:`OnError`
      ;[1 0.2344 0.2344] FAILED operation error
      (`self.FinishTest` "Error" _errormessage))))

(fn `UserConstructionScript`)